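; EnemyProjectile is a flipbook-sprite projectile fired by enemies that damages the player on contact.
; It attaches a fireball trail emitter at spawn and rotates each tick to face its velocity.
; On overlap it ignores enemies, other enemy projectiles and trigger volumes; anything else triggers an ExplodyPuff and destroys it, calling Damage first if it is MyCharacter.
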(event EventTick
  (params (DeltaSeconds :type Float%20%28single-precision%29))
  (Transformation|SetActorRotation (Math|Conversions|RotationFromXVector (Transformation|GetVelocity))))

(event EventBeginPlay
  (Effects|SpawnEmitterAttached "/Game/Effects/FireballTrail.FireballTrail" (Variables|Default|GetTrailAttach) "None" "0, 0, 0" "0, 0, 0" "1.000000,1.000000,1.000000" "SnapToTarget"))

(event Collision|EventActorBeginOverlap
  (params (OtherActor :type Actor%20Object%20Reference))
  (Utilities|Casting|CastToEnemy OtherActor
    (:CastFailed
      (Utilities|Casting|CastToEnemyProjectile OtherActor
        (:CastFailed
          (Utilities|Casting|CastToTriggerVolume OtherActor
            (:CastFailed
              (bind _asmy_character (Utilities|Casting|CastToMyCharacter OtherActor)
                (:then
                  (Default|Damage _asmy_character (Variables|Default|GetDamageAmount)))
                (:CastFailed
                  _))
              (Game|SpawnActorfromClass "/Game/Blueprints/ExplodyPuff.ExplodyPuff_C" (Math|Conversions|ToTransform(Vector) (Transformation|GetActorLocation)) "AdjustIfPossibleButDontSpawnIfColliding" 0 0)
              (Actor|DestroyActor))))))))

(fn ConstructionScript
  (AddComponent|AddPaperFlipbookComponent false (Math|Transform|MakeTransform "-30.000000, 0,5.000000" "0, 0, 0" "1.500000,1.500000,1.500000")))